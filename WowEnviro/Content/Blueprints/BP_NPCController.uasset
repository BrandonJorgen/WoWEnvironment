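; BP_NPCController is an AI controller that makes its NPC either follow the player or turn to face them.
; Each Tick, the Follow flag triggers a move toward the player pawn's location through the NPCMoveTo wrapper around MoveToLocation, stopping within a fixed radius.
; Otherwise, if FacePlayer is set, it snaps the controlled pawn's rotation to look at the player, with no interpolation.
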(event Custom|FollowPlayer
  (CallFunction|NPCMoveto (Transformation|GetActorLocation (Game|Player|GetPlayerPawn 0)) 2e+02))

(event Custom|RotateToFacePlayer
  (bind _returnvalue (Pawn|GetControlledPawn))
  (Transformation|SetActorRotation _returnvalue (Math|Rotator|FindLookatRotation (Transformation|GetActorLocation _returnvalue) (Transformation|GetActorLocation (Game|Player|GetPlayerPawn 0)))))

(event EventTick
  (params (DeltaSeconds :type Float%20%28single-precision%29))
  (if (Variables|Default|GetFollow)
    (CallFunction|FollowPlayer)
    (elif (Variables|Default|GetFacePlayer)
      (CallFunction|RotatetoFacePlayer))))

(fn ConstructionScript)

(fn NPCMoveto
  (params (LocationVector :type Vector) (Acceptance%20Radius :type Float%20%28double-precision%29))
  (bind _returnvalue (AI|Navigation|MovetoLocation LocationVector Acceptance%20Radius true true false true 0))
  (switch Utilities|FlowControl|Switch|SwitchonEPathFollowingRequestResult _returnvalue
    (:AlreadyAtGoal
      _)
    (:RequestSuccessful
      _))
  (return))