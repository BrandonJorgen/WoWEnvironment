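; BP_NPC is a non-player character with a world-space speech bubble for dialogue with the player.
; Hovering the cursor over its mesh changes the player controller's cursor message when the NPC is interactable.
; Enable and disable events toggle the bubble and dialogue state, and another event passes text to the WBP_SpeechBubble widget.
; While dialogue is active, Tick rotates the bubble toward the player's follow camera and the NPC toward the player.
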(event OnBeginCursorOver(Mesh)
  (params (TouchedComponent :type Primitive%20Component%20Object%20Reference))
  (if (Variables|Default|GetNPCInteractable)
    (Class|BPIChangeCursorState|ChangeCursor(Message) (Game|GetPlayerController 0) "NewEnumerator2")))

(event OnEndCursorOver(Mesh)
  (params (TouchedComponent :type Primitive%20Component%20Object%20Reference))
  (Class|BPIChangeCursorState|ChangeCursor(Message) (Game|GetPlayerController 0) "NewEnumerator1"))

(event Custom|EnableSpeechBubble
  (Rendering|SetVisibility (Variables|Default|GetSpeechBubble) true false)
  (Variables|Default|SetDialogueActive true))

(event Custom|DisableSpeechBubble
  (Rendering|SetVisibility (Variables|Default|GetSpeechBubble) false false)
  (Variables|Default|SetDialogueActive false))

(event Custom|ChangeSpeechText
  (params (Text :type Text))
  (Variables|/Game/Blueprints/WBP_SpeechBubble.WBP_SpeechBubble_C|SetNewText (Variables|Default|GetSpeechBubbleWidget) Text))

(event EventTick
  (params (DeltaSeconds :type Float%20%28single-precision%29))
  (bind _returnvalue (Game|Player|GetPlayerPawn 0))
  (bind _speechbubble (Variables|Default|GetSpeechBubble))
  (if (Variables|Default|GetDialogueActive)
    (bind _asbp_mmocharacter (Utilities|Casting|CastToBP_MMOCharacter _returnvalue))
    (Transformation|SetWorldRotation _speechbubble (Math|Rotator|FindLookatRotation (Transformation|GetWorldLocation _speechbubble) (Transformation|GetWorldLocation (Variables|/Game/Blueprints/BP_MMOCharacter.BP_MMOCharacter_C|GetFollowCamera _asbp_mmocharacter))) false false)
    (Transformation|SetActorRotation self (Math|Rotator|FindLookatRotation (Transformation|GetActorLocation) (Transformation|GetActorLocation _returnvalue)))))

(event EventBeginPlay
  (bind _aswbp_speech_bubble (Utilities|Casting|CastToWBP_SpeechBubble (UserInterface|GetWidget (Variables|Default|GetSpeechBubble))))
  (Variables|Default|SetSpeechBubbleWidget _aswbp_speech_bubble))

(fn ConstructionScript)