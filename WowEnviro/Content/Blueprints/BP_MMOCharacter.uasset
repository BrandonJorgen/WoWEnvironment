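; BP_MMOCharacter is a player character with MMO-style movement and camera controls driven by left and right mouse button states.
; Holding right mouse snaps the mesh yaw to the camera and enables strafing; otherwise turn input rotates the mesh, carrying the camera boom along unless left mouse is held.
; Forward movement follows mesh facing and, with neither button held, eases boom yaw toward Arrow2.
; Helper functions handle clamped camera orbit and stepped arm-length zoom.
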(fn ConstructionScript)

(fn RotateCharacterMouse
  (params (RMBDown :type Boolean) (LMBDown :type Boolean) (AxisValue :type Float%20%28double-precision%29))
  (bind _mesh (Variables|Character|GetMesh))
  (if RMBDown
    ;[0 0 0] Right Mouse Button down
    (Transformation|SetWorldRotation _mesh (Math|Rotator|MakeRotator 0.0 0.0 (.yaw (Transformation|GetWorldRotation (Variables|Camera|GetFollowCamera)))) false false)
    (else
      ;[0 0 0] Right Mouse Button NOT down
      (if LMBDown
        (return)
        (else
          ;;[0.2656 0.2656 0.2656] Left Mouse Button NOT down
          (Transformation|AddRelativeRotation _mesh (Math|Rotator|MakeRotator 0.0 0.0 AxisValue) false false)
          (Transformation|AddRelativeRotation (Variables|Camera|GetCameraBoom) (Math|Rotator|MakeRotator 0.0 0.0 AxisValue) false false))))))

(fn RotateCharacterKeyboard
  (params (RMBDown :type Boolean) (LMBDown :type Boolean) (AxisValue :type Float%20%28double-precision%29))
  (bind _mesh (Variables|Character|GetMesh))
  (if RMBDown
    (return)
    (else
      ;[0 0 0] Right Mouse Button NOT down
      (if LMBDown
        ;;[0.2396 0.2396 0.2396] Left Mouse Button down
        (Transformation|AddRelativeRotation _mesh (Math|Rotator|MakeRotator 0.0 0.0 AxisValue) false false)
        (else
          ;;[0.2656 0.2656 0.2656] Left Mouse Button NOT down
          (Transformation|AddRelativeRotation _mesh (Math|Rotator|MakeRotator 0.0 0.0 AxisValue) false false)
          (Transformation|AddRelativeRotation (Variables|Camera|GetCameraBoom) (Math|Rotator|MakeRotator 0.0 0.0 AxisValue) false false))))))

(fn MoveCharacterForward
  (params (AxisValue :type Float%20%28double-precision%29) (RMBDown :type Boolean) (LMBDown :type Boolean))
  (bind _cameraboom (Variables|Camera|GetCameraBoom))
  (bind _relativerotation (Variables|/Script/Engine.SceneComponent|GetRelativeRotation _cameraboom))
  (if (!= AxisValue 0.0)
    (Pawn|Input|AddMovementInput (Math|Vector|GetForwardVector (Variables|Character|GetMesh)) AxisValue false)
    (if LMBDown
      (return)
      (else
        ;[0 0 0] Left Mouse Button NOT down
        (if (not RMBDown)
          ;;[0.1771 0.1771 0.1771] Right Mouse Button NOT down
          (Transformation|SetRelativeRotation _cameraboom (Math|Rotator|MakeRotator (.roll _relativerotation) (.pitch _relativerotation) (.yaw (Math|Rotator|Lerp(Rotator) (Math|Rotator|MakeRotator 0.0 0.0 (.yaw _relativerotation)) (Math|Rotator|MakeRotator 0.0 0.0 (.yaw (Transformation|GetWorldRotation (Variables|Default|GetArrow2)))) 0.03 true))) false false))))
    (else
      (return))))

(fn MoveCharacterStrafe
  (params (AxisValue :type Float%20%28double-precision%29) (RMBDown :type Boolean))
  (if RMBDown
    (Pawn|Input|AddMovementInput (Math|Vector|GetRightVector (Variables|Character|GetMesh)) AxisValue false)
    (else
      (return))))

(fn RotateCamera
  (params (Horizontal :type Float%20%28double-precision%29) (Vertical :type Float%20%28double-precision%29))
  (bind _cameraboom (Variables|Camera|GetCameraBoom))
  (bind _relativerotation (Variables|/Script/Engine.SceneComponent|GetRelativeRotation _cameraboom))
  (bind (_roll _pitch _yaw) (Math|Rotator|BreakRotator _relativerotation))
  (Transformation|SetRelativeRotation _cameraboom (Math|Rotator|MakeRotator 0.0 (Math|Float|Clamp(Float) (+ (* Vertical -1.0) _pitch) -89.0 89.0) (+ Horizontal _yaw)) false false))

(fn ZoomCamera
  (params (ZoomIn :type Boolean))
  (bind _cameraboom (Variables|Camera|GetCameraBoom))
  (if ZoomIn
    (Variables|/Script/Engine.SpringArmComponent|SetTargetArmLength _cameraboom (Math|Float|Clamp(Float) (- (Variables|/Script/Engine.SpringArmComponent|GetTargetArmLength _cameraboom) 35.0) -35.0 1.2e+03))
    (else
      (Variables|/Script/Engine.SpringArmComponent|SetTargetArmLength _cameraboom (Math|Float|Clamp(Float) (+ (Variables|/Script/Engine.SpringArmComponent|GetTargetArmLength _cameraboom) 35.0) -35.0 1.2e+03)))))