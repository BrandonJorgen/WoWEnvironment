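; Charge minigame puzzle where clicking the pedestal activates five three-position switches that route colors through seven conduit arrows.
; Each switch click rotates it 120 degrees, cycles its CurrentKey entry, checks SolutionKey with SkipArray wildcards, then recolors the conduits.
; Hardcoded per-conduit decision trees derive colors from switch states and neighboring conduits, running twice after a null-check pass.
; A match disables interaction and calls the completion dispatcher.
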(event OnBeginCursorOver(Switch1)
  (params (TouchedComponent :type Primitive%20Component%20Object%20Reference))
  (if (Variables|Default|GetMinigameActivated)
    (Class|BPIChangeCursorState|ChangeCursor(Message) (Game|GetPlayerController 0) "NewEnumerator2")))

(event OnBeginCursorOver(Switch2)
  (params (TouchedComponent :type Primitive%20Component%20Object%20Reference))
  (if (Variables|Default|GetMinigameActivated)
    (Class|BPIChangeCursorState|ChangeCursor(Message) (Game|GetPlayerController 0) "NewEnumerator2")))

(event OnClicked(Switch1)
  (params (TouchedComponent :type Primitive%20Component%20Object%20Reference) (ButtonPressed :type Key%20Structure :default "None"))
  (bind _currentkey (Variables|Default|GetCurrentKey))
  (bind _output (Utilities|Array|Get(acopy) _currentkey))
  (if (Variables|Default|GetMinigameActivated)
    (Transformation|AddRelativeRotation (Variables|Default|GetSwitch1) "0,120.000000, 0" false false)
    (if (>= (Utilities|Array|Length _currentkey) 1)
      (if (== _output 2)
        (Utilities|Array|SetArrayElem _currentkey 0 0)
        (else
          (bind _result (Math|Integer|IncrementInt _output)
            (:%20%20
              (Utilities|Array|SetArrayElem _currentkey 0 _result)))))
      (CallFunction|CheckAgainstSolution)
      (CallFunction|UpdateConduits))))

(event OnClicked(Switch2)
  (params (TouchedComponent :type Primitive%20Component%20Object%20Reference) (ButtonPressed :type Key%20Structure :default "None"))
  (bind _currentkey (Variables|Default|GetCurrentKey))
  (bind _output (Utilities|Array|Get(acopy) _currentkey 1))
  (if (Variables|Default|GetMinigameActivated)
    (Transformation|AddRelativeRotation (Variables|Default|GetSwitch2) "0,120.000000, 0" false false)
    (if (>= (Utilities|Array|Length _currentkey) 2)
      (if (== _output 2)
        (Utilities|Array|SetArrayElem _currentkey 1 0)
        (else
          (bind _result (Math|Integer|IncrementInt _output)
            (:%20%20
              (Utilities|Array|SetArrayElem _currentkey 1 _result)))))
      (CallFunction|CheckAgainstSolution)
      (CallFunction|UpdateConduits))))

(event OnClicked(Switch5)
  (params (TouchedComponent :type Primitive%20Component%20Object%20Reference) (ButtonPressed :type Key%20Structure :default "None"))
  (bind _currentkey (Variables|Default|GetCurrentKey))
  (bind _output (Utilities|Array|Get(acopy) _currentkey 2))
  (if (Variables|Default|GetMinigameActivated)
    (Transformation|AddRelativeRotation (Variables|Default|GetSwitch5) "0,120.000000, 0" false false)
    (if (>= (Utilities|Array|Length _currentkey) 3)
      (if (== _output 2)
        (Utilities|Array|SetArrayElem _currentkey 2 0)
        (else
          (bind _result (Math|Integer|IncrementInt _output)
            (:%20%20
              (Utilities|Array|SetArrayElem _currentkey 2 _result)))))
      (CallFunction|CheckAgainstSolution)
      (CallFunction|UpdateConduits))))

(event OnClicked(Switch3)
  (params (TouchedComponent :type Primitive%20Component%20Object%20Reference) (ButtonPressed :type Key%20Structure :default "None"))
  (bind _currentkey (Variables|Default|GetCurrentKey))
  (bind _output (Utilities|Array|Get(acopy) _currentkey 3))
  (if (Variables|Default|GetMinigameActivated)
    (Transformation|AddRelativeRotation (Variables|Default|GetSwitch3) "0,120.000000, 0" false false)
    (if (>= (Utilities|Array|Length _currentkey) 4)
      (if (== _output 2)
        (Utilities|Array|SetArrayElem _currentkey 3 0)
        (else
          (bind _result (Math|Integer|IncrementInt _output)
            (:%20%20
              (Utilities|Array|SetArrayElem _currentkey 3 _result)))))
      (CallFunction|CheckAgainstSolution)
      (CallFunction|UpdateConduits))))

(event OnClicked(Switch4)
  (params (TouchedComponent :type Primitive%20Component%20Object%20Reference) (ButtonPressed :type Key%20Structure :default "None"))
  (bind _currentkey (Variables|Default|GetCurrentKey))
  (bind _output (Utilities|Array|Get(acopy) _currentkey 4))
  (if (Variables|Default|GetMinigameActivated)
    (Transformation|AddRelativeRotation (Variables|Default|GetSwitch4) "0,120.000000, 0" false false)
    (if (>= (Utilities|Array|Length _currentkey) 5)
      (if (== _output 2)
        (Utilities|Array|SetArrayElem _currentkey 4 0)
        (else
          (bind _result (Math|Integer|IncrementInt _output)
            (:%20%20
              (Utilities|Array|SetArrayElem _currentkey 4 _result)))))
      (CallFunction|CheckAgainstSolution)
      (CallFunction|UpdateConduits))))

(event OnClicked(ChargePedestal)
  (params (TouchedComponent :type Primitive%20Component%20Object%20Reference) (ButtonPressed :type Key%20Structure :default "None"))
  (if (Variables|Default|GetMinigameInteractable)
    (if (not (Variables|Default|GetChargePedestalClicked))
      (Variables|Default|SetMinigameActivated true)
      (Variables|Default|SetChargePedestalClicked true)
      (Rendering|SetVisibility (Variables|Default|GetID%20OBject) true false))))

(event OnBeginCursorOver(ChargePedestal)
  (params (TouchedComponent :type Primitive%20Component%20Object%20Reference))
  (if (Variables|Default|GetMinigameInteractable)
    (if (not (Variables|Default|GetChargePedestalClicked))
      (Class|BPIChangeCursorState|ChangeCursor(Message) (Game|GetPlayerController 0) "NewEnumerator2"))))

(event OnEndCursorOver(ChargePedestal)
  (params (TouchedComponent :type Primitive%20Component%20Object%20Reference))
  (Class|BPIChangeCursorState|ChangeCursor(Message) (Game|GetPlayerController 0) "NewEnumerator1"))

(event OnBeginCursorOver(Switch5)
  (params (TouchedComponent :type Primitive%20Component%20Object%20Reference))
  (if (Variables|Default|GetMinigameActivated)
    (Class|BPIChangeCursorState|ChangeCursor(Message) (Game|GetPlayerController 0) "NewEnumerator2")))

(event OnBeginCursorOver(Switch3)
  (params (TouchedComponent :type Primitive%20Component%20Object%20Reference))
  (if (Variables|Default|GetMinigameActivated)
    (Class|BPIChangeCursorState|ChangeCursor(Message) (Game|GetPlayerController 0) "NewEnumerator2")))

(event OnBeginCursorOver(Switch4)
  (params (TouchedComponent :type Primitive%20Component%20Object%20Reference))
  (if (Variables|Default|GetMinigameActivated)
    (Class|BPIChangeCursorState|ChangeCursor(Message) (Game|GetPlayerController 0) "NewEnumerator2")))

(event OnEndCursorOver(Switch1)
  (params (TouchedComponent :type Primitive%20Component%20Object%20Reference))
  (if (Variables|Default|GetMinigameActivated)
    (Class|BPIChangeCursorState|ChangeCursor(Message) (Game|GetPlayerController 0) "NewEnumerator1")))

(event OnEndCursorOver(Switch2)
  (params (TouchedComponent :type Primitive%20Component%20Object%20Reference))
  (if (Variables|Default|GetMinigameActivated)
    (Class|BPIChangeCursorState|ChangeCursor(Message) (Game|GetPlayerController 0) "NewEnumerator1")))

(event OnEndCursorOver(Switch5)
  (params (TouchedComponent :type Primitive%20Component%20Object%20Reference))
  (if (Variables|Default|GetMinigameActivated)
    (Class|BPIChangeCursorState|ChangeCursor(Message) (Game|GetPlayerController 0) "NewEnumerator1")))

(event OnEndCursorOver(Switch3)
  (params (TouchedComponent :type Primitive%20Component%20Object%20Reference))
  (if (Variables|Default|GetMinigameActivated)
    (Class|BPIChangeCursorState|ChangeCursor(Message) (Game|GetPlayerController 0) "NewEnumerator1")))

(event OnEndCursorOver(Switch4)
  (params (TouchedComponent :type Primitive%20Component%20Object%20Reference))
  (if (Variables|Default|GetMinigameActivated)
    (Class|BPIChangeCursorState|ChangeCursor(Message) (Game|GetPlayerController 0) "NewEnumerator1")))

(event Custom|CheckAgainstSolution
  ;[0 0 0] Check solution
  (if (== (Utilities|Array|Length (Variables|Default|GetCurrentKey)) (Utilities|Array|Length (Variables|Default|GetSolutionKey)))
    (bind (_array_element _array_index) (Utilities|Array|ForEachLoopwithBreak (Variables|Default|GetCurrentKey) :!label _label)
      (:LoopBody
        (for (_array_element_2 _array_index_2) (Variables|Default|GetSkipArray)
          (if (== _array_index _array_index_2)
            (if _array_element_2
              _
              (elif (== _array_element (Utilities|Array|Get(acopy) (Variables|Default|GetSolutionKey) _array_index))
                _
                (else
                  (goto _label Break))))
            (Math|Integer|IncrementInt (Variables|Default|GetCorrectCount)))))
      (:Completed
        (if (== (Variables|Default|GetCorrectCount) (Variables|Default|GetSolveCount))
          (Variables|Default|SetMinigameSolved true)
          (CallFunction|MinigameComplete)
          (else
            (Variables|Default|SetCorrectCount 0)))))
    (else
      (Development|PrintString "Solution and Current keys don't share an equal match"))))

(event Custom|UpdateConduits
  (CallFunction|CheckConduits)
  (for (_array_element _array_index) (Variables|Default|GetConduitArray)
    (switch int (Utilities|Array|Get(acopy) (Variables|Default|GetConduitKey) _array_index)
      (:Default
        (Components|Arrow|SetArrowColor(LinearColor) _array_element "(R=1.000000,G=1.000000,B=1.000000,A=1.000000)" :!label _label))
      (:0
        (goto _label))
      (:1
        (Components|Arrow|SetArrowColor(LinearColor) _array_element "(R=1.000000,G=1.000000,B=0.005000,A=1.000000)"))
      (:2
        (Components|Arrow|SetArrowColor(LinearColor) _array_element "(R=1.000000,G=0.000000,B=0.000000,A=1.000000)"))
      (:3
        (Components|Arrow|SetArrowColor(LinearColor) _array_element "(R=0.000000,G=1.000000,B=0.000000,A=1.000000)"))
      (:4
        (Components|Arrow|SetArrowColor(LinearColor) _array_element "(R=0.000000,G=0.000000,B=1.000000,A=1.000000)")))))

(event Custom|CheckConduits
  (Utilities|FlowControl|Sequence
    (:then_0
      _)
    (:then_1
      _))
  (CallFunction|ConduitNullCheck)
  (CallFunction|CheckConduit1)
  (CallFunction|CheckConduit2)
  (CallFunction|CheckConduit3)
  (CallFunction|CheckConduit4)
  (CallFunction|CheckConduit5)
  (CallFunction|CheckConduit6)
  (CallFunction|CheckConduit7))

(event Custom|MinigameComplete
  (Variables|Default|SetMinigameInteractable false)
  (Variables|Default|SetMinigameActivated false)
  (Class|BPIChangeCursorState|ChangeCursor(Message) (Game|GetPlayerController 0) "NewEnumerator1")
  (Rendering|SetVisibility (Variables|Default|GetID%20OBject) false false)
  (Default|CallMinigameCompleteDispatch))

(event EventBeginPlay
  (bind _conduitarray (Variables|Default|GetConduitArray))
  (Variables|Default|SetSolveCount (Utilities|Array|Length (Variables|Default|GetSolutionKey)))
  (Utilities|Array|AddUnique _conduitarray (Variables|Default|GetConduit1))
  (Utilities|Array|AddUnique _conduitarray (Variables|Default|GetConduit2))
  (Utilities|Array|AddUnique _conduitarray (Variables|Default|GetConduit3))
  (Utilities|Array|AddUnique _conduitarray (Variables|Default|GetConduit4))
  (Utilities|Array|AddUnique _conduitarray (Variables|Default|GetConduit5))
  (Utilities|Array|AddUnique _conduitarray (Variables|Default|GetConduit6))
  (Utilities|Array|AddUnique _conduitarray (Variables|Default|GetConduit7))
  (CallFunction|UpdateConduits))

(fn ConstructionScript)

(fn CheckConduit1
  (bind _currentkey (Variables|Default|GetCurrentKey))
  (switch int (Utilities|Array|Get(acopy) _currentkey 1) ; 0 = Red\n1 = Chain, Check Switch 3\n2 = Check Switch 1
    (:0
      (Utilities|Array|SetArrayElem (Variables|Default|GetConduitKey) 0 2)
      (return 2))
    (:1
      (switch int (Utilities|Array|Get(acopy) _currentkey 2) ; 0 = Grey / Check Switch 1\n1 = Grey/ Check Switch 1\n2 = Check Switch 4
        (:0
          _)
        (:1
          _)
        (:2
          (switch int (Utilities|Array|Get(acopy) _currentkey 3) ; 0 = Check Switch 5\n1 = Grey / Check Switch 1\n2 = Green
            (:0
              (switch int (Utilities|Array|Get(acopy) _currentkey 4) ; 0 = Blue\n1 = Grey / Check Switch 1\n2 = Grey / Check Switch 1
                (:0
                  (if (== (Utilities|Array|Get(acopy) (Variables|Default|GetCurrentKey)) 1)
                    (Utilities|Array|SetArrayElem (Variables|Default|GetConduitKey) 0 1)
                    (return 1)
                    (else
                      (Utilities|Array|SetArrayElem (Variables|Default|GetConduitKey) 0 4)
                      (return 4))))
                (:1
                  _)
                (:2
                  _)))
            (:1
              _)
            (:2
              (Utilities|Array|SetArrayElem (Variables|Default|GetConduitKey) 0 3)
              (return 3))))))
    (:2
      _))
  (switch int (Utilities|Array|Get(acopy) _currentkey) ; 0 = Grey\n1 = Yellow\n2 = Grey
    (:0
      _)
    (:1
      (Utilities|Array|SetArrayElem (Variables|Default|GetConduitKey) 0 1)
      (return 1))
    (:2
      _))
  (Utilities|Array|SetArrayElem (Variables|Default|GetConduitKey) 0 0)
  (return 0))

(fn CheckConduit2
  (bind _currentkey (Variables|Default|GetCurrentKey))
  (bind _conduitkey (Variables|Default|GetConduitKey))
  (bind _currentkey_2 (Variables|Default|GetCurrentKey))
  (bind _conduitkey_2 (Variables|Default|GetConduitKey))
  (bind _output (Utilities|Array|Get(acopy) _conduitkey_2 2))
  (bind _output_2 (Utilities|Array|Get(acopy) _currentkey_2 2))
  (bind _returnvalue (== _output_2 2))
  (switch int (Utilities|Array|Get(acopy) _currentkey 1) ; 0 = Grey / Check Switch 3\n1 = Chain, Check Switch 1\n2 = Red
    (:0
      (switch int (Utilities|Array|Get(acopy) _currentkey 2) ; 0 = Check Switch 1\n1 = Check Switch 1\n2 = Grey / Check Switch 4
        (:0
          _)
        (:1
          _)
        (:2
          (switch int (Utilities|Array|Get(acopy) _currentkey 3) ; 0 = Chain, Check Switch 5\n1 = Grey\n2 = Green
            (:0
              (switch int (Utilities|Array|Get(acopy) _currentkey 4) ; 0 = Blue\n1 = Grey\n2 = Grey
                (:0
                  (Utilities|Array|SetArrayElem (Variables|Default|GetConduitKey) 1 4)
                  (return 4))
                (:1
                  _)
                (:2
                  _))
              (Utilities|Array|SetArrayElem (Variables|Default|GetConduitKey) 1 0)
              (return 0))
            (:1
              (Utilities|Array|SetArrayElem (Variables|Default|GetConduitKey) 1 0)
              (return 0))
            (:2
              (Utilities|Array|SetArrayElem (Variables|Default|GetConduitKey) 1 3)
              (return 3))))))
    (:1
      _)
    (:2
      (Utilities|Array|SetArrayElem (Variables|Default|GetConduitKey) 1 2)
      (return 2)))
  (switch int (Utilities|Array|Get(acopy) _currentkey) ; 0 = Grey / Check Switch 3\n1 = Yellow\n2 = Grey / Check Switch 3
    (:0
      _)
    (:1
      (if (and (== (Utilities|Array|Get(acopy) _currentkey_2 3) 2) _returnvalue)
        (Utilities|Array|SetArrayElem _conduitkey 1 3)
        (return 3)
        (elif (== (Utilities|Array|Get(acopy) _currentkey_2 1) 1)
          (Utilities|Array|SetArrayElem _conduitkey 1 1)
          (return 1)
          (else
            (Utilities|Array|SetArrayElem _conduitkey 1 0)
            (return 0)))))
    (:2
      _))
  (if _returnvalue
    (Utilities|Array|SetArrayElem _conduitkey 1 _output)
    (return _output)
    (else
      (Utilities|Array|SetArrayElem _conduitkey 1 0)
      (return 0))))

(fn ConduitNullCheck
  (bind _conduitkey (Variables|Default|GetConduitKey))
  (bind _conduitkey_2 (Variables|Default|GetConduitKey))
  (bind _conduitkey_3 (Variables|Default|GetConduitKey))
  (bind _currentkey (Variables|Default|GetCurrentKey))
  (bind _conduitkey_4 (Variables|Default|GetConduitKey))
  (bind _output (Utilities|Array|Get(acopy) _currentkey 1))
  (for (_ _array_index) (Variables|Default|GetConduitKey)
    (switch int _array_index
      (:1
        ;[1 1 0] Yellow
        (if (not (== (Utilities|Array|Get(acopy) (Variables|Default|GetCurrentKey)) 1))
          (for (_array_element _array_index_2) _conduitkey
            (if (== _array_element 1)
              (Utilities|Array|SetArrayElem _conduitkey _array_index_2 0)))))
      (:2
        ;[1 0 0] Red
        (if (not (or (== _output 0) (== _output 2)))
          (for (_array_element_2 _array_index_3) _conduitkey_3
            (if (== _array_element_2 2)
              (Utilities|Array|SetArrayElem _conduitkey_3 _array_index_3 0)))))
      (:3
        ;[0 1 0] Green
        (if (not (== (Utilities|Array|Get(acopy) (Variables|Default|GetCurrentKey) 3) 1))
          (for (_array_element_3 _array_index_4) _conduitkey_2
            (if (== _array_element_3 3)
              (Utilities|Array|SetArrayElem _conduitkey_2 _array_index_4 0)))))
      (:4
        ;[0 0 1] Blue
        (if (not (== (Utilities|Array|Get(acopy) (Variables|Default|GetCurrentKey) 4) 0))
          (for (_array_element_4 _array_index_5) _conduitkey_4
            (if (== _array_element_4 4)
              (Utilities|Array|SetArrayElem _conduitkey_4 _array_index_5 0)))))))
  (return))

(fn CheckConduit3
  (bind _currentkey (Variables|Default|GetCurrentKey))
  (bind _currentkey_2 (Variables|Default|GetCurrentKey))
  (bind _conduitkey (Variables|Default|GetConduitKey))
  (bind _conduitkey_2 (Variables|Default|GetConduitKey))
  (bind _output (Utilities|Array|Get(acopy) _currentkey 2))
  (bind _output_2 (Utilities|Array|Get(acopy) _conduitkey 1))
  (bind _output_3 (Utilities|Array|Get(acopy) _conduitkey_2 1))
  (switch int (Utilities|Array|Get(acopy) _currentkey 3) ; 0 = Check Switch 3\n1 = Check Switch 3\n2 = Green
    (:0
      (switch int _output ; 0 = Check Switch 5\n1 = Check Switch 5\n2 = Check Switch 2
        (:0
          _)
        (:1
          _)
        (:2
          (switch int (Utilities|Array|Get(acopy) _currentkey 1) :!label _label ; 0 = Grey\n1 = Check Switch 1\n2 = Red
            (:0
              (if (== (Utilities|Array|Get(acopy) (Variables|Default|GetCurrentKey) 4) 0)
                (Utilities|Array|SetArrayElem (Variables|Default|GetConduitKey) 2 4)
                (return 4)
                (else
                  (Utilities|Array|SetArrayElem (Variables|Default|GetConduitKey) 2 0)
                  (return 0))))
            (:1
              (switch int (Utilities|Array|Get(acopy) _currentkey) ; 0 = Check Switch 5\n1 = Yellow\n0 = Check Switch 5
                (:0
                  _)
                (:1
                  (if (and (== (Utilities|Array|Get(acopy) _currentkey_2 4) 0) (== (Utilities|Array|Get(acopy) _currentkey_2 3) 0))
                    (Utilities|Array|SetArrayElem (Variables|Default|GetConduitKey) 2 4)
                    (return 4)
                    (else
                      (Utilities|Array|SetArrayElem _conduitkey 2 _output_2)
                      (return _output_2))))
                (:2
                  _)))
            (:2
              (Utilities|Array|SetArrayElem (Variables|Default|GetConduitKey) 2 2)
              (return 2)))))
      (switch int (Utilities|Array|Get(acopy) _currentkey 4) ; 0 = Blue\n1 = Grey\n2 = Grey
        (:0
          _)
        (:1
          (Utilities|Array|SetArrayElem (Variables|Default|GetConduitKey) 2 0 :!label _label_2)
          (return 0))
        (:2
          (goto _label_2))))
    (:1
      (switch int _output ; 0 = Grey\n1 = Grey\n2 = Check Switch 2
        (:0
          (goto _label_2))
        (:1
          (goto _label_2))
        (:2
          (goto _label))))
    (:2
      (Utilities|Array|SetArrayElem (Variables|Default|GetConduitKey) 2 3)
      (return 3)))
  (if (== (Utilities|Array|Get(acopy) (Variables|Default|GetCurrentKey) 3) 0)
    (Utilities|Array|SetArrayElem (Variables|Default|GetConduitKey) 2 4)
    (return 4)
    (else
      (Utilities|Array|SetArrayElem _conduitkey_2 2 _output_3)
      (return _output_3))))

(fn CheckConduit4
  (bind _currentkey (Variables|Default|GetCurrentKey))
  (bind _conduitkey (Variables|Default|GetConduitKey))
  (switch int (Utilities|Array|Get(acopy) _currentkey 3) ; 0 = Check Switch 3\n1= Green\n2 = Check Switch 5
    (:0
      (switch int (Utilities|Array|Get(acopy) _currentkey 2) ; 0 = Check Switch 5\n1 = Check Switch 5\n2 = Check Switch 2
        (:0
          _)
        (:1
          _)
        (:2
          (switch int (Utilities|Array|Get(acopy) _currentkey 1) ; 0 = Check Switch 5\n1 = Check Switch 1\n2 = Red
            (:0
              _)
            (:1
              (switch int (Utilities|Array|Get(acopy) _currentkey) ; 0 = Grey\n1 = Yellow\n2 = Grey
                (:0
                  (if (== (Utilities|Array|Get(acopy) (Variables|Default|GetCurrentKey) 4) 0)
                    (Utilities|Array|SetArrayElem _conduitkey 3 4)
                    (return 4)
                    (else
                      _)))
                (:1
                  (Utilities|Array|SetArrayElem (Variables|Default|GetConduitKey) 3 1)
                  (return 1))
                (:2
                  _))
              (Utilities|Array|SetArrayElem _conduitkey 3 0)
              (return 0))
            (:2
              (Utilities|Array|SetArrayElem (Variables|Default|GetConduitKey) 3 2)
              (return 2))))))
    (:1
      (Utilities|Array|SetArrayElem (Variables|Default|GetConduitKey) 3 3)
      (return 3))
    (:2
      _))
  (switch int (Utilities|Array|Get(acopy) _currentkey 4) ; 0 = Blue\n1 = Grey\n2 = Grey
    (:0
      (Utilities|Array|SetArrayElem (Variables|Default|GetConduitKey) 3 4)
      (return 4))
    (:1
      _)
    (:2
      _))
  (Utilities|Array|SetArrayElem (Variables|Default|GetConduitKey) 3 0)
  (return 0))

(fn CheckConduit5
  (bind _currentkey (Variables|Default|GetCurrentKey))
  (switch int (Utilities|Array|Get(acopy) _currentkey) ; 0 = Check Switch 2\n1 = Grey\n2 = Yellow
    (:0
      (switch int (Utilities|Array|Get(acopy) _currentkey 1) ; 0 = Red\n1 = Grey\n2 = Grey
        (:0
          (Utilities|Array|SetArrayElem (Variables|Default|GetConduitKey) 4 2)
          (return 2))
        (:1
          _)
        (:2
          _)))
    (:1
      _)
    (:2
      (Utilities|Array|SetArrayElem (Variables|Default|GetConduitKey) 4 1)
      (return 1)))
  (Utilities|Array|SetArrayElem (Variables|Default|GetConduitKey) 4 0)
  (return 0))

(fn CheckConduit6
  (bind _currentkey (Variables|Default|GetCurrentKey))
  (switch int (Utilities|Array|Get(acopy) _currentkey 2) ; 0 = Check Switch 2\n1 = Check Switch 4\n2 = Grey
    (:0
      (switch int (Utilities|Array|Get(acopy) _currentkey 1) ; 0 = Grey\n1 = Grey\n2 = Red
        (:0
          _)
        (:1
          _)
        (:2
          (Utilities|Array|SetArrayElem (Variables|Default|GetConduitKey) 5 2)
          (return 2)))
      (Utilities|Array|SetArrayElem (Variables|Default|GetConduitKey) 5 0)
      (return 0))
    (:1
      (switch int (Utilities|Array|Get(acopy) _currentkey 3) ; 0 = Grey\n1 = Grey\n2 = Green
        (:0
          _)
        (:1
          _)
        (:2
          (Utilities|Array|SetArrayElem (Variables|Default|GetConduitKey) 5 3)
          (return 3)))
      (Utilities|Array|SetArrayElem (Variables|Default|GetConduitKey) 5 0)
      (return 0))
    (:2
      (Utilities|Array|SetArrayElem (Variables|Default|GetConduitKey) 5 0)
      (return 0))))

(fn CheckConduit7
  (bind _currentkey (Variables|Default|GetCurrentKey))
  (switch int (Utilities|Array|Get(acopy) _currentkey 4) ; 0 = Grey\n1 = Check Switch 4\n2 = Blue
    (:0
      (Utilities|Array|SetArrayElem (Variables|Default|GetConduitKey) 6 0)
      (return 0))
    (:1
      (switch int (Utilities|Array|Get(acopy) _currentkey 3) ; 0 = Grey\n1 = Green\n2 = Grey
        (:0
          _)
        (:1
          (Utilities|Array|SetArrayElem (Variables|Default|GetConduitKey) 6 3)
          (return 3))
        (:2
          _))
      (Utilities|Array|SetArrayElem (Variables|Default|GetConduitKey) 6 0)
      (return 0))
    (:2
      (Utilities|Array|SetArrayElem (Variables|Default|GetConduitKey) 6 4)
      (return 4))))